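; Player controller for the ArenaBattle game that manages the HUD and end-of-game presentation.
; On BeginPlay it creates the HUD, caches its score widget and sets the clear score from BP_ABGameMode.
; Events forward score and retry-count changes to that widget.
; Game over and game clear both show a result widget with a success flag, and a clear also spawns BP_Congratulation at the pawn's location.
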(event Custom|OnNewScore
  (Default|SetScore (Variables|Default|GetScoreWidget) (stale EventOnScoreChanged NewScore)))

(event Custom|OnGameOver
  (Variables|Default|SetIsSuccess false)
  (bind _returnvalue (UserInterface|CreateWidget "/Game/ArenaBattle/UI/WBP_GameResult.WBP_GameResult_C" (Game|GetPlayerController 0)))
  (UserInterface|Viewport|AddtoViewport _returnvalue 0)
  (Default|SetResult _returnvalue (Variables|Default|GetIsSuccess)))

(event Custom|OnGameClear
  (Variables|Default|SetIsSuccess true)
  (Utilities|FlowControl|Sequence
    (:then_0
      (bind _returnvalue (UserInterface|CreateWidget "/Game/ArenaBattle/UI/WBP_GameResult.WBP_GameResult_C" (Game|GetPlayerController 0)))
      (UserInterface|Viewport|AddtoViewport _returnvalue 0)
      (Default|SetResult _returnvalue (Variables|Default|GetIsSuccess)))
    (:then_1
      (Game|SpawnActorfromClass "/Game/ArenaBattle/Blueprint/BP_Congratulation.BP_Congratulation_C" (Math|Conversions|ToTransform(Vector) (Transformation|GetActorLocation (Pawn|GetControlledPawn))) "Undefined" 0 0))))

(event EventBeginPlay
  (bind _returnvalue (UserInterface|CreateWidget "/Game/ArenaBattle/UI/WBP_ABHUD.WBP_ABHUD_C"))
  (UserInterface|Viewport|AddtoViewport _returnvalue 0) ; Add to Viewport 로 화면에 띄우기
  (Variables|Default|SetScoreWidget (Variables|/Game/ArenaBattle/UI/WBP_ABHUD.WBP_ABHUD_C|GetWBP_PlayerScore _returnvalue))
  (bind _asbp_abgame_mode (Utilities|Casting|CastToBP_ABGameMode (Game|GetGameMode)))
  (Default|SetClearScore (Variables|Default|GetScoreWidget) (Variables|/Script/UnrealArenaBattle.ABGameMode|GetClearScore _asbp_abgame_mode)))

(event EventOnGameRetryCount
  (params (NewRetryCount :type Integer))
  (Default|SetRetryCount (Variables|Default|GetScoreWidget) NewRetryCount))

(event EventOnScoreChanged
  (params (NewScore :type Integer))
  (Default|SetScore (Variables|Default|GetScoreWidget) NewScore))

(event EventOnGameOver
  (Variables|Default|SetIsSuccess false)
  (bind _returnvalue (UserInterface|CreateWidget "/Game/ArenaBattle/UI/WBP_GameResult.WBP_GameResult_C" (Game|GetPlayerController 0)))
  (UserInterface|Viewport|AddtoViewport _returnvalue 0)
  (Default|SetResult _returnvalue (Variables|Default|GetIsSuccess)))

(event EventOnGameClear
  (Variables|Default|SetIsSuccess true)
  (Utilities|FlowControl|Sequence
    (:then_0
      (bind _returnvalue (UserInterface|CreateWidget "/Game/ArenaBattle/UI/WBP_GameResult.WBP_GameResult_C" (Game|GetPlayerController 0)))
      (UserInterface|Viewport|AddtoViewport _returnvalue 0)
      (Default|SetResult _returnvalue (Variables|Default|GetIsSuccess)))
    (:then_1
      (Game|SpawnActorfromClass "/Game/ArenaBattle/Blueprint/BP_Congratulation.BP_Congratulation_C" (Math|Conversions|ToTransform(Vector) (Transformation|GetActorLocation (Pawn|GetControlledPawn))) "Undefined" 0 0))))

(fn ConstructionScript)